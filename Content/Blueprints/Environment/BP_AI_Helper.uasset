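; Placed patrol point helper for AI, identified by patrol group and point number, that tracks whether it is vacant.
; Overlap events keep a list of characters inside; an NPC entering clears Vacant, and one leaving restores it only if the list is empty.
; The construction script labels the point with its group and number; its visual components are hidden on play.
; Debug mode tracks the overlapping player for a camera-facing function, which is empty.
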(event EventBeginPlay
  (Rendering|SetVisibility (Variables|Default|GetDefaultSceneRoot) false false))

(event Collision|EventActorBeginOverlap
  (params (OtherActor :type Actor%20Object%20Reference))
  (Variables|Default|SetOtherActorBeginOverlap OtherActor)
  (Utilities|Casting|CastToBP_CharacterBase (Variables|Default|GetOtherActorBeginOverlap))
  (Utilities|Array|AddUnique (Variables|Default|GetOverlappedActors) (Variables|Default|GetOtherActorBeginOverlap))
  (Utilities|FlowControl|Sequence
    (:then_0
      (if (Variables|Default|GetDebug)
        (bind _asbp_player_character (Utilities|Casting|CastToBP_PlayerCharacter (Variables|Default|GetOtherActorBeginOverlap)))
        (Variables|Default|SetOverlappedPlayer _asbp_player_character)
        (Variables|Default|SetIsLookAtPlayerCamera true)))
    (:then_1
      (Utilities|Casting|CastToBP_NPCCharacters (Variables|Default|GetOtherActorBeginOverlap))
      (Variables|Default|SetVacant false))))

(event EventTick
  (params (DeltaSeconds :type Float%20%28single-precision%29))
  (if (Variables|Default|GetDebug)
    (CallFunction|LookingatPlayerCamera)))

(event Collision|EventActorEndOverlap
  (params (OtherActor :type Actor%20Object%20Reference))
  (Variables|Default|SetOtherActorEndOverlap OtherActor)
  (Utilities|Casting|CastToBP_CharacterBase (Variables|Default|GetOtherActorEndOverlap))
  (bind _returnvalue (Utilities|Array|RemoveItem (Variables|Default|GetOverlappedActors) (Variables|Default|GetOtherActorEndOverlap)))
  (if _returnvalue
    (Utilities|FlowControl|Sequence
      (:then_0
        (if (Variables|Default|GetDebug)
          (Utilities|Casting|CastToBP_PlayerCharacter (Variables|Default|GetOtherActorEndOverlap))
          (Variables|Default|SetOverlappedPlayer 0)
          (Variables|Default|SetIsLookAtPlayerCamera false)))
      (:then_1
        (Utilities|Casting|CastToBP_NPCCharacters (Variables|Default|GetOtherActorEndOverlap))
        (if (Utilities|Array|IsValidIndex (Variables|Default|GetOverlappedActors))
          (Variables|Default|SetVacant false)
          (else
            (Variables|Default|SetVacant true)))))))

(fn ConstructionScript
  (if (!= (Variables|Default|GetPatrollGroup) 0)
    (Rendering|Components|TextRender|SetText (Variables|Default|GetTextRender) (Utilities|Text|FormatText "Group {A} : Point {B}" (Variables|Default|GetPatrollGroup) (Variables|Default|GetPatrollPointNumber)))
    (else
      (Rendering|Components|TextRender|SetText (Variables|Default|GetTextRender) (Utilities|Text|FormatText "Set patroll group")))))

(fn LookingatPlayerCamera)