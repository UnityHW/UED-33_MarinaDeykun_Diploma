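; BP_PushableObject is a pushable environment object that the player latches onto when running into it.
; On a hit from the player character, it stores the player's rounded forward vector as PushableDirection.
; CanPush then runs a short line trace from the player along their facing to confirm this object is in front.
; If so, it disables player movement and attaches the player to itself, though it contains no movement logic.
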(event EventBeginPlay)

(event Collision|EventActorBeginOverlap
  (params (OtherActor :type Actor%20Object%20Reference)))

(event EventTick
  (params (DeltaSeconds :type Float%20%28single-precision%29)))

(event Collision|EventHit
  (params (MyComp :type Primitive%20Component%20Object%20Reference) (Other :type Actor%20Object%20Reference) (OtherComp :type Primitive%20Component%20Object%20Reference) (bSelfMoved :type Boolean) (HitLocation :type Vector :default "0, 0, 0") (HitNormal :type Vector :default "0, 0, 0") (NormalImpulse :type Vector :default "0, 0, 0") (Hit :type Hit%20Result%20Structure%20%28by%20ref%29))
  (bind _returnvalue (Transformation|GetActorForwardVector Other))
  (bind _returnvalue_2 (Game|GetPlayerCharacter 0))
  (bind (_x _y _z) (Math|Vector|BreakVector _returnvalue))
  (if (== (Game|GetPlayerCharacter 0) Other)
    (Variables|Default|SetPushableDirection (Math|Vector|MakeVector (Math|Conversions|ToFloat(Integer) (Math|Float|Round _x)) (Math|Conversions|ToFloat(Integer) (Math|Float|Round _y)) (Math|Conversions|ToFloat(Integer) (Math|Float|Round _z))))
    (bind _canpush (CallFunction|CanPush))
    (if _canpush
      (Pawn|Components|CharacterMovement|DisableMovement (Variables|/Script/Engine.Character|GetCharacterMovement _returnvalue_2))
      (Transformation|AttachActorToActor _returnvalue_2 self "None" "KeepWorld" "KeepWorld" "KeepWorld" true))))

(fn ConstructionScript)

(fn CanPush
  (bind _returnvalue (Game|GetPlayerCharacter 0))
  (bind _returnvalue_2 (Transformation|GetActorLocation _returnvalue))
  (bind (_outhit _returnvalue_3) (Collision|LineTraceByChannel _returnvalue_2 (+ _returnvalue_2 (* (Transformation|GetActorForwardVector _returnvalue) 1e+02)) "TraceTypeQuery1" false (Utilities|Array|MakeArray _returnvalue) "None"))
  (if _returnvalue_3
    (if (== (.HitActor (Collision|BreakHitResult _outhit)) self)
      (return true)
      (else
        (return false)))
    (else
      (return false))))