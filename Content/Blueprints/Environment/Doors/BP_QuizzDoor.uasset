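; Puzzle door that moves vertically once a required number of pressure switches are active at the same time.
; Activate and deactivate events raise or lower a switch counter and compare it to the needed count.
; Meeting the count plays a timeline that drives the door mesh's relative Z location, while falling short reverses the same timeline.
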(event Custom|PressureSwitchActivated
  (Math|Integer|IncrementInt (Variables|Default|GetPressureSwitchesActive)
    (:%20%20
      (if (>= (Variables|Default|GetPressureSwitchesActive) (Variables|Default|GetPressureSwitchesNeeded))
        (bind _quizzdorrposition (Timeline|QuizzDoorActivation Play)
          (:Update
            (Transformation|SetRelativeLocation (Variables|Default|GetQuizzDoorMesh) (Math|Vector|MakeVector 0.0 0.0 _quizzdorrposition) false false)))
        (else
          (Timeline|QuizzDoorActivation Reverse))))))

(event Custom|PressureSwitchDeactivated
  (Math|Integer|DecrementInt (Variables|Default|GetPressureSwitchesActive)
    (:%20%20
      (if (>= (Variables|Default|GetPressureSwitchesActive) (Variables|Default|GetPressureSwitchesNeeded))
        (bind _quizzdorrposition (Timeline|QuizzDoorActivation Play)
          (:Update
            (Transformation|SetRelativeLocation (Variables|Default|GetQuizzDoorMesh) (Math|Vector|MakeVector 0.0 0.0 _quizzdorrposition) false false)))
        (else
          (Timeline|QuizzDoorActivation Reverse))))))

(event EventBeginPlay)

(event Collision|EventActorBeginOverlap
  (params (OtherActor :type Actor%20Object%20Reference)))

(event EventTick
  (params (DeltaSeconds :type Float%20%28single-precision%29)))

(fn ConstructionScript)