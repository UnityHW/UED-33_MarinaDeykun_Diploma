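; NPC character Blueprint with a health bar, name label, weapon aiming and simple player interaction.
; Each tick, a player-distance check gates the health bar, hidden when line-of-sight is blocked, and a camera-facing debug label showing name and AI state.
; While shooting and chasing, the weapon smoothly rotates toward the AI controller's target.
; Neutral or friendly NPCs detect the player through an interact sphere and show random phrase pop-ups on interaction.
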(event OnComponentBeginOverlap(InteractSphere)
  (params (OverlappedComponent :type Primitive%20Component%20Object%20Reference) (OtherActor :type Actor%20Object%20Reference) (OtherComp :type Primitive%20Component%20Object%20Reference) (OtherBodyIndex :type Integer) (bFromSweep :type Boolean) (SweepResult :type Hit%20Result%20Structure%20%28by%20ref%29))
  (switch Utilities|FlowControl|Switch|SwitchonENUM_Fractions (Variables|/Game/Blueprints/Components/BP_MainStatsComponent.BP_MainStatsComponent_C|GetCurrentFraction (Variables|Default|GetBP_MainStatsComponent))
    (:NewEnumerator1
      _)
    (:NewEnumerator2
      _))
  (bind _asbp_player_character (Utilities|Casting|CastToBP_PlayerCharacter OtherActor))
  (Variables|Default|SetPlayerCharacterInBox _asbp_player_character)
  (if (not (Variables|/Game/Blueprints/Components/BP_MainStatsComponent.BP_MainStatsComponent_C|GetIsDead (Variables|Default|GetBP_MainStatsComponent)))
    (Rendering|SetVisibility (Variables|Default|GetInfoScene) true true)
    (Variables|Default|SetIsReadyToInteract true)))

(event OnComponentEndOverlap(InteractSphere)
  (params (OverlappedComponent :type Primitive%20Component%20Object%20Reference) (OtherActor :type Actor%20Object%20Reference) (OtherComp :type Primitive%20Component%20Object%20Reference) (OtherBodyIndex :type Integer))
  (Utilities|Casting|CastToBP_PlayerCharacter OtherActor)
  (Variables|Default|SetPlayerCharacterInBox 0)
  (Rendering|SetVisibility (Variables|Default|GetInfoScene) false true)
  (Variables|Default|SetIsReadyToInteract false))

(event EventBeginPlay
  (|CallParentFunction)
  (Utilities|FlowControl|Sequence
    (:then_0
      (bind _asw_health_bar (Utilities|Casting|CastToW_HealthBar (UserInterface|GetUserWidgetObject (Variables|Default|GetWidgetHP))))
      (Default|UpdateCurrentCharacterforHP _asw_health_bar self))
    (:then_1
      (Rendering|SetVisibility (Variables|Default|GetTooltipText) (Variables|Default|GetDebug) true))))

(event Collision|EventActorBeginOverlap
  (params (OtherActor :type Actor%20Object%20Reference))
  (|CallParentFunction OtherActor) ; This node is disabled and will not be called.\nDrag off pins to build functionality.
)

(event EventTick
  (params (DeltaSeconds :type Float%20%28single-precision%29))
  (|CallParentFunction DeltaSeconds)
  ;[1 1 1] looking at the player camera ADD
  (Variables|Default|SetIsLookAtPlayerCamera (<= (Math|Vector|VectorLength (- (Transformation|GetWorldLocation (Variables|Default|GetCapsuleComponent)) (Transformation|GetActorLocation (Game|Player|GetPlayerPawn 0)))) 1.5e+03))
  (CallFunction|LookingatPlayerCamera)
  (CallFunction|UpdateInfoWighetVisibility))

(fn ConstructionScript
  (bind _bp_mainstatscomponent (Variables|Default|GetBP_MainStatsComponent))
  (bind _currentmane (Variables|/Game/Blueprints/Components/BP_MainStatsComponent.BP_MainStatsComponent_C|GetCurrentMane _bp_mainstatscomponent))
  (|CallParentFunction)
  (if (Utilities|Name|NotEqual(Name) _currentmane "None")
    (Rendering|Components|TextRender|SetText (Variables|Default|GetTooltipText) (Utilities|Text|FormatText "{Name}" _currentmane))
    (else
      (Rendering|Components|TextRender|SetText (Variables|Default|GetTooltipText) (Utilities|Text|FormatText "SET NAME FOR NPC!!!!!!")))))

(fn UpdatePatrollingGroup
  (params (InPatrollingGroup :type Byte))
  ;[1 1 1] CHECK
  (Variables|Default|SetPatrollingGroup InPatrollingGroup)
  (if (>= (Variables|Default|GetPatrollingGroup) 0)
    ;[1 1 1] Update AI State patrolling
    (Utilities|Casting|CastToBP_AIController (AI|GetAIController self))))

(fn ActionMain
  (params (IsPressed :type Boolean))
  (|CallParentFunction IsPressed)
  (if (Variables|Default|GetIsActionMainPressed)
    (Development|PrintString "Bang" true false "(R=0.950000,G=0.000000,B=0.395312,A=1.000000)" 1.0)))

(fn LookingatPlayerCamera
  (if (Variables|Default|GetIsLookAtPlayerCamera)
    (bind _asbp_aicontroller (Utilities|Casting|CastToBP_AIController (Pawn|GetController)))
    (Variables|/Game/Blueprints/Controllers/BP_AIController.BP_AIController_C|GetTargetCharacter _asbp_aicontroller
      (:then
        (bind _asbp_player_character (Utilities|Casting|CastToBP_PlayerCharacter (Game|Player|GetPlayerPawn 0)))
        (LocalVariables|SetL_CameraLocation (Transformation|GetWorldLocation (Variables|/Game/Blueprints/Characters/Player/BP_PlayerCharacter.BP_PlayerCharacter_C|GetCamera _asbp_player_character)))
        (Rendering|Components|TextRender|SetText (Variables|Default|GetTooltipText) (Utilities|Text|FormatText "{Name} | {AIState}" (Utilities|String|EnumtoString (Variables|/Game/Blueprints/Controllers/BP_AIController.BP_AIController_C|GetAIState _asbp_aicontroller)) (Variables|/Game/Blueprints/Components/BP_MainStatsComponent.BP_MainStatsComponent_C|GetCurrentMane (Variables|Default|GetBP_MainStatsComponent))))
        (Transformation|SetWorldRotation (Variables|Default|GetTooltipText) (Math|Rotator|FindLookatRotation (Transformation|GetWorldLocation (Variables|Default|GetInfoScene)) (LocalVariables|GetL_CameraLocation)) false false))
      (:else))))

(fn UpdateWidgetVisibility)

(fn UpdateWeaponSceneRotation
  (|CallParentFunction)
  (bind _currentweapon (Variables|Default|GetCurrentWeapon)
    (:then
      (switch Utilities|FlowControl|Switch|SwitchonENUM_WeaponState (Variables|/Game/Blueprints/Weapons/BP_WeaponBase.BP_WeaponBase_C|GetWeaponState _currentweapon)
        (:NewEnumerator1
          (bind _asbp_aicontroller (Utilities|Casting|CastToBP_AIController (Pawn|GetController)))
          (switch Utilities|FlowControl|Switch|SwitchonENUM_AIStates (Variables|/Game/Blueprints/Controllers/BP_AIController.BP_AIController_C|GetAIState _asbp_aicontroller)
            (:NewEnumerator3
              (bind _targetcharacter (Variables|/Game/Blueprints/Controllers/BP_AIController.BP_AIController_C|GetTargetCharacter _asbp_aicontroller)
                (:then
                  (LocalVariables|SetL_TargetLocation (Transformation|GetActorLocation _targetcharacter))
                  (Transformation|SetWorldRotation (Variables|Default|GetWeaponScene) (Math|Rotator|MakeRotator 0.0 (.Pitch (Math|Rotator|BreakRotator (Math|Interpolation|RInterpTo (Transformation|GetWorldRotation (Variables|Default|GetWeaponScene)) (Math|Rotator|FindLookatRotation (Transformation|GetWorldLocation (Variables|Default|GetWeaponScene)) (LocalVariables|GetL_TargetLocation)) (Utilities|Time|GetWorldDeltaSeconds) 1e+01))) (.Yaw (Math|Rotator|BreakRotator (Math|Interpolation|RInterpTo (Transformation|GetWorldRotation (Variables|Default|GetWeaponScene)) (Math|Rotator|FindLookatRotation (Transformation|GetWorldLocation (Variables|Default|GetWeaponScene)) (LocalVariables|GetL_TargetLocation)) (Utilities|Time|GetWorldDeltaSeconds) 1e+01)))) false false))
                (:else)))))))
    (:else)))

(fn UpdateInfoWighetVisibility
  (if (Variables|Default|GetIsLookAtPlayerCamera)
    (if (not (Variables|/Game/Blueprints/Components/BP_MainStatsComponent.BP_MainStatsComponent_C|GetIsDead (Variables|Default|GetBP_MainStatsComponent)))
      (bind _asbp_player_character (Utilities|Casting|CastToBP_PlayerCharacter (Game|Player|GetPlayerPawn 0)))
      (bind _returnvalue (Collision|LineTraceByChannel (Transformation|GetWorldLocation (Variables|Default|GetWidgetHP)) (Transformation|GetWorldLocation (Variables|/Game/Blueprints/Characters/Player/BP_PlayerCharacter.BP_PlayerCharacter_C|GetCamera _asbp_player_character)) "TraceTypeQuery1" true (Utilities|Array|MakeArray self) "None"))
      (Rendering|SetVisibility (Variables|Default|GetWidgetHP) (not _returnvalue) false))
    (else
      (Rendering|SetVisibility (Variables|Default|GetWidgetHP) false false))))

(fn AddPopUptotheViewport
  (params (InText :type Text))
  (Variables|Default|GetPlayerCharacterInBox
    (:then
      (bind _asplayer_controller (Utilities|Casting|CastToPlayerController (Pawn|GetController (Variables|Default|GetPlayerCharacterInBox))))
      (bind _returnvalue (UserInterface|CreateWidget "/Game/Blueprints/HUD/Widgets/W_PopUp.W_PopUp_C" _asplayer_controller self InText))
      (Variables|Default|SetCurrentPopUp _returnvalue)
      (UserInterface|Viewport|AddtoViewport (Variables|Default|GetCurrentPopUp) 0)
      (UserInterface|Animation|PlayAnimation (Variables|Default|GetCurrentPopUp) (Variables|/Game/Blueprints/HUD/Widgets/W_PopUp.W_PopUp_C|GetMoveAndFade (Variables|Default|GetCurrentPopUp)) 0.0 1 "Forward" 1.0 false))
    (:else)))

(fn Interact
  (if (Variables|Default|GetIsReadyToInteract)
    (Utilities|FlowControl|Sequence
      (:then_0
        (if (Utilities|Array|IsValidIndex (Variables|Default|GetPhrasesForPopUps))
          (CallFunction|AddPopUptotheViewport (Utilities|Array|Get(acopy) (Variables|Default|GetPhrasesForPopUps) (Math|Random|RandomIntegerinRange 0 (- (Utilities|Array|Length (Variables|Default|GetPhrasesForPopUps)) 1))))))
      (:then_1
        (return true)))
    (else
      (return true))))