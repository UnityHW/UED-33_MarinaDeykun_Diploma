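; Backpack component that holds a character's quest items, consumables and owned weapons, with reserve ammo mapped by weapon name.
; On BeginPlay it restores all three from the GameInstance's save object, only for the player character outside a new game.
; Ammo updates clamp using the current weapon's stats, notify that weapon and return a round count; adding a weapon also updates the character's current weapon.
; Consumable add/remove functions are empty stubs.
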(event EventBeginPlay
  (CallFunction|ConfigureBackpack))

(event EventTick
  (params (DeltaSeconds :type Float%20%28single-precision%29)))

(fn AddQuestItem
  (params (InItemName :type Name))
  (Utilities|Set|Add (Variables|Default|GetQuestItems) InItemName))

(fn RemoveQuestItem
  (params (InItemName :type Name))
  (bind _returnvalue (Utilities|Set|Remove (Variables|Default|GetQuestItems) InItemName))
  (return _returnvalue))

(fn AddConsumableItem)

(fn RemoveConsumableItem)

(fn UpdateAmmobyName
  (params (InAmmo :type Integer) (InIncreased :type Boolean) (InWeaponName :type Name))
  (bind _availableweapon_ (Variables|Default|GetAvailableWeapon%20))
  (bind (_value _returnvalue) (Utilities|Map|Find _availableweapon_ InWeaponName))
  (bind _asbp_character_base (Utilities|Casting|CastToBP_CharacterBase (Components|GetOwner)))
  (bind _currentweapon (Variables|/Game/Blueprints/Characters/BP_CharacterBase.BP_CharacterBase_C|GetCurrentWeapon _asbp_character_base)
    (:then
      (LocalVariables|SetL_CurrentWeapon _currentweapon)
      (if _returnvalue
        (LocalVariables|SetL_AmmoInBackpackCurrent _value)
        (Utilities|FlowControl|Sequence
          (:then_0
            (if InIncreased
              (Utilities|FlowControl|Sequence
                (:then_0
                  (if (<= (LocalVariables|GetL_AmmoInBackpackCurrent) 0)
                    (if (<= (Variables|/Game/Blueprints/Weapons/BP_WeaponBase.BP_WeaponBase_C|GetRoundCurrent (LocalVariables|GetL_CurrentWeapon)) 0)
                      (Variables|/Game/Blueprints/Weapons/BP_WeaponBase.BP_WeaponBase_C|SetWeaponState (LocalVariables|GetL_CurrentWeapon) "NewEnumerator2"))))
                (:then_1
                  (LocalVariables|SetL_Current (+ (LocalVariables|GetL_AmmoInBackpackCurrent) InAmmo))
                  (if (< (LocalVariables|GetL_Current) (.AmmoInBackpackMax (Utilities|Struct|BreakSTRUCT_WeaponStats (Variables|/Game/Blueprints/Weapons/BP_WeaponBase.BP_WeaponBase_C|GetWeaponStats (LocalVariables|GetL_CurrentWeapon)))))
                    (LocalVariables|SetL_AmmoInBackpackCurrent (LocalVariables|GetL_Current))
                    (else
                      (LocalVariables|SetL_AmmoInBackpackCurrent (.AmmoInBackpackMax (Utilities|Struct|BreakSTRUCT_WeaponStats (Variables|/Game/Blueprints/Weapons/BP_WeaponBase.BP_WeaponBase_C|GetWeaponStats (LocalVariables|GetL_CurrentWeapon)))))))))
              (else
                (LocalVariables|SetL_Current (- (LocalVariables|GetL_AmmoInBackpackCurrent) InAmmo))
                (if (> (LocalVariables|GetL_Current) 0)
                  (LocalVariables|SetL_AmmoInBackpackCurrent (LocalVariables|GetL_Current))
                  (LocalVariables|SetL_Current (.RoundsMax (Utilities|Struct|BreakSTRUCT_WeaponStats (Variables|/Game/Blueprints/Weapons/BP_WeaponBase.BP_WeaponBase_C|GetWeaponStats (LocalVariables|GetL_CurrentWeapon)))))
                  (else
                    (LocalVariables|SetL_AmmoInBackpackCurrent 0)
                    (LocalVariables|SetL_Current (+ (.RoundsMax (Utilities|Struct|BreakSTRUCT_WeaponStats (Variables|/Game/Blueprints/Weapons/BP_WeaponBase.BP_WeaponBase_C|GetWeaponStats (LocalVariables|GetL_CurrentWeapon)))) (LocalVariables|GetL_Current))))))))
          (:then_1
            (Utilities|Map|Add (Variables|Default|GetAvailableWeapon%20) InWeaponName (LocalVariables|GetL_AmmoInBackpackCurrent)))
          (:then_2
            (Default|CallOnWeaponStatusChanged (LocalVariables|GetL_CurrentWeapon))
            (return (LocalVariables|GetL_Current))))
        (else
          (Default|CallOnWeaponStatusChanged (LocalVariables|GetL_CurrentWeapon))
          (return 0))))
    (:else)))

(fn Debug
  (bind _values (Utilities|Map|Values (Variables|Default|GetAvailableWeapon%20)))
  (for _array_element _values
    (Variables|Default|SetL_String (Utilities|String|Append (Variables|Default|GetL_String) " | " (Utilities|String|ToString(Integer) _array_element))))
  (Development|PrintString (Variables|Default|GetL_String) true true "(R=0.000000,G=0.660000,B=1.000000,A=1.000000)" 0.0))

(fn GetAmmoforWeapon
  (params (InWeaponName :type Name%20%28by%20ref%29))
  (bind _availableweapon_ (Variables|Default|GetAvailableWeapon%20))
  (bind (_value _returnvalue) (Utilities|Map|Find _availableweapon_ InWeaponName))
  (if _returnvalue
    (return true _value)
    (else
      (return false 0))))

(fn GetMaxRoundsforWeapon
  (params (InWeaponName :type Name))
  (bind _returnvalue (Utilities|GetDataTableRow "/Game/Data/DT_WeaponStats.DT_WeaponStats" InWeaponName)
    (:then
      (return true (Utilities|Struct|BreakSTRUCT_WeaponStats _returnvalue)))
    (:RowNotFound
      (return false 0))))

(fn AddWeaponItem
  (params (InWeaponName :type Name))
  (Utilities|Map|Add (Variables|Default|GetAvailableWeapon%20) InWeaponName 0)
  (bind _asbp_character_base (Utilities|Casting|CastToBP_CharacterBase (Components|GetOwner)))
  (Default|UpdateCurrentWeapon _asbp_character_base InWeaponName))

(fn ConfigureBackpack
  (bind _savegameobject (Utilities|CheckSaveGame)
    (:Is%20Valid
      (LocalVariables|SetL_Save _savegameobject)
      (Utilities|FlowControl|Sequence
        (:then_0
          (Variables|Default|SetQuestItems (Variables|/Game/Blueprints/Objects/BP_SaveGame.BP_SaveGame_C|GetSavedQuestItems (LocalVariables|GetL_Save))))
        (:then_1
          (Variables|Default|SetConsumableItems (Variables|/Game/Blueprints/Objects/BP_SaveGame.BP_SaveGame_C|GetSavedConsumableItems (LocalVariables|GetL_Save))))
        (:then_2
          (Variables|Default|SetAvailableWeapon%20 (Variables|/Game/Blueprints/Objects/BP_SaveGame.BP_SaveGame_C|GetSavedAvailableWeapon%20 (LocalVariables|GetL_Save))))))))